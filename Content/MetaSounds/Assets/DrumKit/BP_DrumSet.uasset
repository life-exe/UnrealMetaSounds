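; BP_DrumSet is a drum kit actor that plays a MetaSound and animates its drum pieces in sync, starting and stopping as a Character enters or leaves its box trigger.
; BeginPlay labels it with the sound's name and maps eight child BP_Drum actors by name.
; The MetaSound Output Subsystem watches an output per map key, and each reported output calls Play on the matching drum.
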(event OnComponentBeginOverlap(Box)
  (params (OverlappedComponent :type Primitive%20Component%20Object%20Reference) (OtherActor :type Actor%20Object%20Reference) (OtherComp :type Primitive%20Component%20Object%20Reference) (OtherBodyIndex :type Integer) (bFromSweep :type Boolean) (SweepResult :type Hit%20Result%20Structure%20%28by%20ref%29))
  (if (Class|GameplayStatics|ObjectIsA OtherActor "/Script/Engine.Character")
    (Components|Activation|Activate (Variables|Default|GetAudio) false)))

(event OnComponentEndOverlap(Box)
  (params (OverlappedComponent :type Primitive%20Component%20Object%20Reference) (OtherActor :type Actor%20Object%20Reference) (OtherComp :type Primitive%20Component%20Object%20Reference) (OtherBodyIndex :type Integer))
  (if (Class|GameplayStatics|ObjectIsA OtherActor "/Script/Engine.Character")
    (Components|Activation|Deactivate (Variables|Default|GetAudio))))

(event Custom|OnOutput
  (params (OutputName :type Name) (Output :type Meta%20Sound%20Output%20Structure%20%28by%20ref%29))
  (bind _drums (Variables|Default|GetDrums))
  (bind (_value _returnvalue) (Utilities|Map|Find _drums OutputName))
  (if _returnvalue
    (Default|Play _value)))

(event EventBeginPlay
  (Rendering|Components|TextRender|SetText (Variables|Default|GetTextRender) (Utilities|Text|ToText(String) (Utilities|GetDisplayName (Variables|/Script/Engine.AudioComponent|GetSound (Variables|Default|GetAudio)))))
  (Utilities|Map|Add (Variables|Default|GetDrums) "HiHat" (.AsBP%20Drum (Utilities|Casting|CastToBP_Drum (Variables|/Script/Engine.ChildActorComponent|GetChildActor (Variables|Default|GetHiHat)))))
  (Utilities|Map|Add (Variables|Default|GetDrums) "Tom1" (.AsBP%20Drum (Utilities|Casting|CastToBP_Drum (Variables|/Script/Engine.ChildActorComponent|GetChildActor (Variables|Default|GetHIghTom)))))
  (Utilities|Map|Add (Variables|Default|GetDrums) "Floor" (.AsBP%20Drum (Utilities|Casting|CastToBP_Drum (Variables|/Script/Engine.ChildActorComponent|GetChildActor (Variables|Default|GetFloor)))))
  (Utilities|Map|Add (Variables|Default|GetDrums) "Crash" (.AsBP%20Drum (Utilities|Casting|CastToBP_Drum (Variables|/Script/Engine.ChildActorComponent|GetChildActor (Variables|Default|GetCrash)))))
  (Utilities|Map|Add (Variables|Default|GetDrums) "Kick" (.AsBP%20Drum (Utilities|Casting|CastToBP_Drum (Variables|/Script/Engine.ChildActorComponent|GetChildActor (Variables|Default|GetKick)))))
  (Utilities|Map|Add (Variables|Default|GetDrums) "Tom2" (.AsBP%20Drum (Utilities|Casting|CastToBP_Drum (Variables|/Script/Engine.ChildActorComponent|GetChildActor (Variables|Default|GetLowTom)))))
  (Utilities|Map|Add (Variables|Default|GetDrums) "Ride" (.AsBP%20Drum (Utilities|Casting|CastToBP_Drum (Variables|/Script/Engine.ChildActorComponent|GetChildActor (Variables|Default|GetRide)))))
  (Utilities|Map|Add (Variables|Default|GetDrums) "Snare" (.AsBP%20Drum (Utilities|Casting|CastToBP_Drum (Variables|/Script/Engine.ChildActorComponent|GetChildActor (Variables|Default|GetSnare)))))
  (bind _keys (Utilities|Map|Keys (Variables|Default|GetDrums)))
  (for _array_element _keys
    (MetaSoundOutput|WatchOutput (WorldSubsystems|GetMetaSoundOutputSubsystem) (Variables|Default|GetAudio) _array_element (delegate Custom|OnOutput) "None" "None" :!class /Script/MetasoundEngine.MetaSoundOutputSubsystem)))

(fn ConstructionScript)