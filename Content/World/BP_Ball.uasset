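; BP_Ball is a ball actor that gets a random size at spawn and makes an explosion sound when it hits anything other than a Pawn.
; BeginPlay stores a random uniform scale and applies it to the Sphere.
; The first qualifying hit disables further hit notifications, starts a short lifespan, and plays the MSExplosion audio with a "Bang" trigger and the scale as its "Size" parameter.
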(event EventBeginPlay
  (bind _output_get (Variables|Default|SetScale (Math|Random|RandomFloatinRange 0.3 1.0)))
  (Transformation|SetWorldScale3D (Variables|Default|GetSphere) (Math|Vector|MakeVector _output_get _output_get _output_get)))

(event Collision|EventHit
  (params (MyComp :type Primitive%20Component%20Object%20Reference) (Other :type Actor%20Object%20Reference) (OtherComp :type Primitive%20Component%20Object%20Reference) (bSelfMoved :type Boolean) (HitLocation :type Vector :default "0, 0, 0") (HitNormal :type Vector :default "0, 0, 0") (NormalImpulse :type Vector :default "0, 0, 0") (Hit :type Hit%20Result%20Structure%20%28by%20ref%29))
  (bind _ms_explosion (Variables|Default|GetMS_Explosion))
  (if (not (Class|GameplayStatics|ObjectIsA Other "/Script/Engine.Pawn"))
    (Actor|SetLifeSpan 5.0)
    (Class|PrimitiveComponent|SetNotifyRigidBodyCollision (Variables|Default|GetSphere) false)
    (Audio|Components|Audio|Play _ms_explosion 0.0)
    (Class|AudioParameterControllerInterface|SetTriggerParameter _ms_explosion "Bang")
    (Audio|Parameter|SetFloatParameter _ms_explosion "Size" (Variables|Default|GetScale) :!class /Script/AudioExtensions.AudioParameterControllerInterface)))

(fn ConstructionScript)